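; Player hero with two-wheel steering: left or right input turns it, both together drive it forward while the wheels spin.
; Inputs ramp up clamped speeds, which custom per-tick loop macros decay into coasting; the stop input blocks movement and speeds up decay.
; The camera has clamped free look.
; Overlapping a BPI_Items actor enables interact, which spawns a copy at ItemPlayer, destroys the original and clears the Pickup flag.
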(event OnComponentBeginOverlap(CollCam)
  (params (OverlappedComponent :type Primitive%20Component%20Object%20Reference) (OtherActor :type Actor%20Object%20Reference) (OtherComp :type Primitive%20Component%20Object%20Reference) (OtherBodyIndex :type Integer) (bFromSweep :type Boolean) (SweepResult :type Hit%20Result%20Structure%20%28by%20ref%29))
  (if (Utilities|DoesObjectImplementInterface OtherActor "/Game/BP/Items/BPI_Items.BPI_Items_C")
    (if (Variables|Default|GetPickup?)
      (Utilities|FlowControl|Gate true) ; enters at Open
    )))

(event OnComponentEndOverlap(CollCam)
  (params (OverlappedComponent :type Primitive%20Component%20Object%20Reference) (OtherActor :type Actor%20Object%20Reference) (OtherComp :type Primitive%20Component%20Object%20Reference) (OtherBodyIndex :type Integer))
  (if (Utilities|DoesObjectImplementInterface OtherActor "/Game/BP/Items/BPI_Items.BPI_Items_C")
    (if (Variables|Default|GetPickup?)
      (Utilities|FlowControl|Gate true) ; enters at Close
    )))

(event Custom|E_TouchMapping
  (bind _returnvalue (Game|GetPlayerController 0))
  (bind _returnvalue_2 (PlayerController|LocalPlayerSubsystems|GetEnhancedInputLocalPlayerSubsystem _returnvalue))
  ;[1 1 1] Begin
  (Utilities|IsValid _returnvalue_2
    (:Is%20Valid
      (Input|AddMappingContext _returnvalue_2 "/Game/BP/Hero/Input/IMC_Hero.IMC_Hero" 0 "(bIgnoreAllPressedKeysUntilRelease=True,bForceImmediately=False,bNotifyUserSettings=False)"))))

(event Custom|E_DrawCursor
  (bind _returnvalue (UserInterface|CreateWidget "/Game/Widget/Cursor/W_CursorPlayer.W_CursorPlayer_C"))
  (bind _output_get (Variables|Default|SetCursorRef _returnvalue))
  (UserInterface|Viewport|AddtoViewport _output_get 0))

(event Custom|E_TurnRight
  ;[0.1203 1 0] Move
  (bind _value (Utilities|MLoopFor+ (Variables|Move|GetRightMove) (Variables|Move|GetSubstract))
    (:Loop
      (bind _output_get (Variables|Move|SetRightMove _value))
      (Utilities|MTurnPlayer _output_get
        (:Exec
          (bind _output_get_2 (Variables|WheelAnim|SetRotateWheelR (+ (Variables|WheelAnim|GetRotateWheelR) (stale Input|EnhancedActionEvents|EnhancedInputActionIA_RightMove _output_get_6))))
          (if (<= _output_get_2 -3.6e+02)
            (Variables|WheelAnim|SetRotateWheelR 0.0))
          (Transformation|SetRelativeRotation (Variables|Default|GetPointWheelR) (Math|Rotator|MakeRotator 0.0 (Variables|WheelAnim|GetRotateWheelR) 0.0) false false))))))

(event Custom|E_TurnLeft
  ;[0.1203 1 0] Move
  (bind _value (Utilities|MLoopFor- (Variables|Move|GetLeftMove) (Variables|Move|GetSubstract))
    (:Loop
      (bind _output_get (Variables|Move|SetLeftMove _value))
      (Utilities|MTurnPlayer _output_get
        (:Exec
          (bind _output_get_2 (Variables|WheelAnim|SetRotateWheelL (- (Variables|WheelAnim|GetRotateWheelL) (stale Input|EnhancedActionEvents|EnhancedInputActionIA_LeftMove _output_get_3))))
          (if (<= _output_get_2 -3.6e+02)
            (Variables|WheelAnim|SetRotateWheelL 0.0))
          (Transformation|SetRelativeRotation (Variables|Default|GetPointWheelL) (Math|Rotator|MakeRotator 0.0 (Variables|WheelAnim|GetRotateWheelL) 0.0) false false))))))

(event Custom|E_ForwardMove
  ;[0.1203 1 0] Move
  (bind _value (Utilities|MLoopFor-Forward (Variables|Move|GetForwardMove) (Variables|Move|GetSubstractForward))
    (:Loop
      (bind _output_get (Variables|Move|SetForwardMove _value))
      (Pawn|Input|AddMovementInput (Math|Rotator|GetRotationXVector (Transformation|GetActorRotation)) _output_get false)
      (Utilities|FlowControl|Sequence
        (:then_0
          (bind _output_get_2 (Variables|WheelAnim|SetRotateWheelL (- (Variables|WheelAnim|GetRotateWheelL) (Variables|Move|GetForwardMove))))
          (if (<= _output_get_2 -3.6e+02)
            (Variables|WheelAnim|SetRotateWheelL 0.0))
          (Transformation|SetRelativeRotation (Variables|Default|GetPointWheelL) (Math|Rotator|MakeRotator 0.0 (Variables|WheelAnim|GetRotateWheelL) 0.0) false false))
        (:then_1
          (bind _output_get_3 (Variables|WheelAnim|SetRotateWheelR (- (Variables|WheelAnim|GetRotateWheelR) (Variables|Move|GetForwardMove))))
          (if (<= _output_get_3 -3.6e+02)
            (Variables|WheelAnim|SetRotateWheelR 0.0))
          (Transformation|SetRelativeRotation (Variables|Default|GetPointWheelR) (Math|Rotator|MakeRotator 0.0 (Variables|WheelAnim|GetRotateWheelR) 0.0) false false))))))

(event Input|EnhancedActionEvents|EnhancedInputActionIA_CameraMove
  (params (ActionValue :type Vector%202D%20Structure) (ElapsedSeconds :type Float%20%28double-precision%29) (TriggeredSeconds :type Float%20%28double-precision%29) (InputAction :type Input%20Action%20Object%20Reference :default "/Game/BP/Hero/Input/Action/IA_CameraMove.IA_CameraMove"))
  ;[0.04979 1 0] Cam Move
  (Utilities|FlowControl|Sequence
    (:then_0
      (bind _output_get (Variables|Move|SetYaw (Math|Float|Clamp(Float) (+ (Variables|Move|GetYaw) (.x ActionValue)) -9e+01 9e+01))))
    (:then_1
      (bind _output_get_2 (Variables|Move|SetPitch (Math|Float|Clamp(Float) (+ (Variables|Move|GetPitch) (.y ActionValue)) -6e+01 6e+01)))))
  (Transformation|SetRelativeRotation (Variables|Default|GetCamera) (Math|Rotator|MakeRotator 0.0 _output_get_2 _output_get) false false))

(event Input|EnhancedActionEvents|EnhancedInputActionIA_LeftMove
  (params (ActionValue :type Boolean) (ElapsedSeconds :type Float%20%28double-precision%29) (TriggeredSeconds :type Float%20%28double-precision%29) (InputAction :type Input%20Action%20Object%20Reference :default "/Game/BP/Hero/Input/Action/IA_LeftMove.IA_LeftMove"))
  ;[0.1203 1 0] Move
  (:Triggered
    (if (Variables|Move|GetOkMove?)
      (Variables|Move|SetLeftM? true)
      (Utilities|FlowControl|Sequence
        (:then_0
          (Utilities|FlowControl|Gate true :!label _label
            (:Exit
              (if (Variables|Move|GetRightM?)
                (Utilities|FlowControl|Sequence
                  (:then_0
                    (Utilities|FlowControl|Gate true) ; enters at Open
                  )
                  (:then_1
                    (Utilities|FlowControl|DoOnce false :!label _label_2
                      (:Completed
                        (bind _value (Utilities|MLoopFor- (Variables|Move|GetLeftMove) (Variables|Move|GetSubstract) :!label _label_3)
                          (:Loop
                            (bind _output_get (Variables|Move|SetLeftMove _value))
                            (Utilities|MTurnPlayer _output_get
                              (:Exec
                                (bind _output_get_2 (Variables|WheelAnim|SetRotateWheelL (- (Variables|WheelAnim|GetRotateWheelL) (stale _output_get_3)) :!label _label_4))
                                (if (<= _output_get_2 -3.6e+02)
                                  (Variables|WheelAnim|SetRotateWheelL 0.0))
                                (Transformation|SetRelativeRotation (Variables|Default|GetPointWheelL) (Math|Rotator|MakeRotator 0.0 (Variables|WheelAnim|GetRotateWheelL) 0.0) false false)))))))))
                (else
                  (Utilities|FlowControl|Sequence
                    (:then_0
                      (if (Variables|Move|GetStopSpeedLeft)
                        (bind _output_get_3 (Variables|Move|SetLeftMove (Math|Float|Clamp(Float) (+ (Variables|Move|GetLeftMove) 0.004) 0.0 0.4)))
                        (if (>= _output_get_3 0.39)
                          (Utilities|FlowControl|Sequence
                            (:then_0
                              (Variables|Move|SetStopSpeedLeft false)
                              (CallFunction|ETurnLeft))
                            (:then_1
                              (Utilities|FlowControl|Delay 1.0)
                              (Variables|Move|SetStopSpeedLeft true)
                              (goto _label_5 Open))
                            (:then_2
                              (goto _label_5 Close)))
                          (else
                            (Utilities|FlowControl|Gate false :!label _label_5
                              (:Exit
                                (Utilities|MTurnPlayer _output_get_3
                                  (:Exec
                                    (goto _label_4)))))))))
                    (:then_1
                      (if (Variables|Move|GetStopSpeedLeft)
                        (goto _label_3 Break)))
                    (:then_2
                      (goto _label_2 Reset))))))))
        (:then_1
          (Utilities|FlowControl|Delay 0.2)
          (goto _label Open)))))
  (:Completed
    (Variables|Move|SetLeftM? false)
    (Utilities|FlowControl|Sequence
      (:then_0
        (if (Variables|Move|GetForwardM?)
          (Utilities|FlowControl|Sequence
            (:then_0
              (Utilities|FlowControl|Gate true) ; enters at Close
            )
            (:then_1
              (if (Variables|Move|GetForwardM?)
                (Variables|Move|SetForwardM? false)
                (bind _value_2 (Utilities|MLoopFor-Forward (Variables|Move|GetForwardMove) (Variables|Move|GetSubstractForward))
                  (:Loop
                    (bind _output_get_4 (Variables|Move|SetForwardMove _value_2))
                    (Pawn|Input|AddMovementInput (Math|Rotator|GetRotationXVector (Transformation|GetActorRotation)) _output_get_4 false)
                    (Utilities|FlowControl|Sequence
                      (:then_0
                        (bind _output_get_5 (Variables|WheelAnim|SetRotateWheelL (- (Variables|WheelAnim|GetRotateWheelL) (Variables|Move|GetForwardMove))))
                        (if (<= _output_get_5 -3.6e+02)
                          (Variables|WheelAnim|SetRotateWheelL 0.0))
                        (Transformation|SetRelativeRotation (Variables|Default|GetPointWheelL) (Math|Rotator|MakeRotator 0.0 (Variables|WheelAnim|GetRotateWheelL) 0.0) false false))
                      (:then_1
                        (bind _output_get_6 (Variables|WheelAnim|SetRotateWheelR (- (Variables|WheelAnim|GetRotateWheelR) (Variables|Move|GetForwardMove))))
                        (if (<= _output_get_6 -3.6e+02)
                          (Variables|WheelAnim|SetRotateWheelR 0.0))
                        (Transformation|SetRelativeRotation (Variables|Default|GetPointWheelR) (Math|Rotator|MakeRotator 0.0 (Variables|WheelAnim|GetRotateWheelR) 0.0) false false))))))))
          (else
            (goto _label_3))))
      (:then_1
        (goto _label Close)))))

(event Input|EnhancedActionEvents|EnhancedInputActionIA_RightMove
  (params (ActionValue :type Boolean) (ElapsedSeconds :type Float%20%28double-precision%29) (TriggeredSeconds :type Float%20%28double-precision%29) (InputAction :type Input%20Action%20Object%20Reference :default "/Game/BP/Hero/Input/Action/IA_RightMove.IA_RightMove"))
  ;[0.1203 1 0] Move
  (:Triggered
    (if (Variables|Move|GetOkMove?)
      (Variables|Move|SetRightM? true)
      (Utilities|FlowControl|Sequence
        (:then_0
          (Utilities|FlowControl|Gate true :!label _label
            (:Exit
              (if (Variables|Move|GetLeftM?)
                (Utilities|FlowControl|Sequence
                  (:then_0
                    (Utilities|FlowControl|Gate true :!label _label_2
                      (:Exit
                        (Variables|Move|SetForwardM? true)
                        (Utilities|FlowControl|Sequence
                          (:then_0
                            (if (Variables|Move|GetStopSpeedForward)
                              (bind _output_get (Variables|Move|SetForwardMove (Math|Float|Clamp(Float) (+ (Variables|Move|GetForwardMove) 0.02))))
                              (if (> _output_get 0.9)
                                (Utilities|FlowControl|Sequence
                                  (:then_0
                                    (Variables|Move|SetStopSpeedForward false)
                                    (CallFunction|EForwardMove))
                                  (:then_1
                                    (Utilities|FlowControl|Delay 1.0)
                                    (Variables|Move|SetStopSpeedForward true)
                                    (goto _label_3 Open))
                                  (:then_2
                                    (goto _label_3 Close)))
                                (else
                                  (Utilities|FlowControl|Gate false :!label _label_3
                                    (:Exit
                                      (Pawn|Input|AddMovementInput (Math|Rotator|GetRotationXVector (Transformation|GetActorRotation)) _output_get false)
                                      (Utilities|FlowControl|Sequence :!label _label_4
                                        (:then_0
                                          (bind _output_get_2 (Variables|WheelAnim|SetRotateWheelL (- (Variables|WheelAnim|GetRotateWheelL) (Variables|Move|GetForwardMove))))
                                          (if (<= _output_get_2 -3.6e+02)
                                            (Variables|WheelAnim|SetRotateWheelL 0.0))
                                          (Transformation|SetRelativeRotation (Variables|Default|GetPointWheelL) (Math|Rotator|MakeRotator 0.0 (Variables|WheelAnim|GetRotateWheelL) 0.0) false false))
                                        (:then_1
                                          (bind _output_get_3 (Variables|WheelAnim|SetRotateWheelR (- (Variables|WheelAnim|GetRotateWheelR) (Variables|Move|GetForwardMove))))
                                          (if (<= _output_get_3 -3.6e+02)
                                            (Variables|WheelAnim|SetRotateWheelR 0.0))
                                          (Transformation|SetRelativeRotation (Variables|Default|GetPointWheelR) (Math|Rotator|MakeRotator 0.0 (Variables|WheelAnim|GetRotateWheelR) 0.0) false false)))))))))
                          (:then_1
                            (if (Variables|Move|GetStopSpeedForward)
                              (goto _label_9 Break)))))))
                  (:then_1
                    (Utilities|FlowControl|DoOnce false :!label _label_5
                      (:Completed
                        (bind _value (Utilities|MLoopFor+ (Variables|Move|GetRightMove) (Variables|Move|GetSubstract) :!label _label_6)
                          (:Loop
                            (bind _output_get_4 (Variables|Move|SetRightMove _value))
                            (Utilities|MTurnPlayer _output_get_4
                              (:Exec
                                (bind _output_get_5 (Variables|WheelAnim|SetRotateWheelR (+ (Variables|WheelAnim|GetRotateWheelR) (stale _output_get_6)) :!label _label_7))
                                (if (<= _output_get_5 -3.6e+02)
                                  (Variables|WheelAnim|SetRotateWheelR 0.0))
                                (Transformation|SetRelativeRotation (Variables|Default|GetPointWheelR) (Math|Rotator|MakeRotator 0.0 (Variables|WheelAnim|GetRotateWheelR) 0.0) false false)))))))))
                (else
                  (Utilities|FlowControl|Sequence
                    (:then_0
                      (if (Variables|Move|GetStopSpeedR)
                        (bind _output_get_6 (Variables|Move|SetRightMove (Math|Float|Clamp(Float) (- (Variables|Move|GetRightMove) 0.004) -0.4 0.0)))
                        (if (<= _output_get_6 -0.39)
                          (Utilities|FlowControl|Sequence
                            (:then_0
                              (Variables|Move|SetStopSpeedR false)
                              (CallFunction|ETurnRight))
                            (:then_1
                              (Utilities|FlowControl|Delay 1.0)
                              (Variables|Move|SetStopSpeedR true)
                              (goto _label_8 Open))
                            (:then_2
                              (goto _label_8 Close)))
                          (else
                            (Utilities|FlowControl|Gate false :!label _label_8
                              (:Exit
                                (Utilities|MTurnPlayer _output_get_6
                                  (:Exec
                                    (goto _label_7)))))))))
                    (:then_1
                      (if (Variables|Move|GetStopSpeedR)
                        (goto _label_6 Break)))
                    (:then_2
                      (goto _label_5 Reset))))))))
        (:then_1
          (Utilities|FlowControl|Delay 0.2)
          (goto _label Open)))))
  (:Completed
    (Variables|Move|SetRightM? false)
    (Utilities|FlowControl|Sequence
      (:then_0
        (if (Variables|Move|GetForwardM?)
          (Utilities|FlowControl|Sequence
            (:then_0
              (goto _label_2 Close))
            (:then_1
              (if (Variables|Move|GetForwardM?)
                (Variables|Move|SetForwardM? false)
                (bind _value_2 (Utilities|MLoopFor-Forward (Variables|Move|GetForwardMove) (Variables|Move|GetSubstractForward) :!label _label_9)
                  (:Loop
                    (bind _output_get_7 (Variables|Move|SetForwardMove _value_2))
                    (Pawn|Input|AddMovementInput (Math|Rotator|GetRotationXVector (Transformation|GetActorRotation)) _output_get_7 false)
                    (goto _label_4))))))
          (else
            (goto _label_6))))
      (:then_1
        (goto _label Close)))))

(event Input|EnhancedActionEvents|EnhancedInputActionIA_Interact
  (params (ActionValue :type Boolean) (ElapsedSeconds :type Float%20%28double-precision%29) (TriggeredSeconds :type Float%20%28double-precision%29) (InputAction :type Input%20Action%20Object%20Reference :default "/Game/BP/Hero/Input/Action/IA_Interact.IA_Interact"))
  (:Started
    (Utilities|FlowControl|Gate true
      (:Exit
        (Variables|Default|SetActor%20Ref (stale OnComponentBeginOverlap(CollCam) OtherActor))
        (CallFunction|FPickItems (stale OnComponentBeginOverlap(CollCam) OtherActor))
        (Actor|DestroyActor (Variables|Default|GetActor%20Ref))
        (Utilities|FlowControl|Delay 0.2)
        (Variables|Default|SetActor%20Ref 0)))))

(event Input|EnhancedActionEvents|EnhancedInputActionIA_StopMove
  (params (ActionValue :type Boolean) (ElapsedSeconds :type Float%20%28double-precision%29) (TriggeredSeconds :type Float%20%28double-precision%29) (InputAction :type Input%20Action%20Object%20Reference :default "/Game/BP/Hero/Input/Action/IA_StopMove.IA_StopMove"))
  ;[0.1203 1 0] Move
  (:Triggered
    (Variables|Move|SetSubstract 0.006)
    (Variables|Move|SetSubstractForward 0.008)
    (Variables|Move|SetOkMove? false))
  (:Completed
    (Variables|Move|SetSubstract 0.002)
    (Variables|Move|SetSubstractForward 0.004)
    (Variables|Move|SetOkMove? true)))

(event EventBeginPlay
  ;[1 1 1] Begin
  (Utilities|FlowControl|Sequence
    (:then_0
      (CallFunction|ETouchMapping)
      (CallFunction|EDrawCursor))))

(fn ConstructionScript)

(fn FPickItems
  (params (Object :type Actor%20Object%20Reference))
  (Variables|Default|SetPickup? false)
  (Game|SpawnActorfromClass (Utilities|GetClass Object) (Transformation|GetWorldTransform (Variables|Default|GetItemPlayer)) "Undefined" "MultiplyWithRoot" self 0)
  (Collision|SetActorEnableCollision false)
  (Transformation|AttachComponentToComponent (Variables|Default|GetItemPlayer) "None" "SnapToTarget" "SnapToTarget" "SnapToTarget" true))