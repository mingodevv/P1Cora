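; PC_Hero is the hero's player controller, handling switching between the pause menu and options menu.
; Each open event clears all widgets, creates and stores a new W_Option or W_Pause in the viewport, then clears the other stored menu's flag if that reference is valid.
; A separate event clears all widgets and removes both stored menus from their parents.
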(event Custom|OptionOpenMenuE
  (bind _refpause (Variables|Default|GetRefPause))
  (Viewport|RemoveAllWidgets)
  (bind _returnvalue (UserInterface|CreateWidget "/Game/Widget/Menu/W_Option.W_Option_C" self))
  (bind _output_get (Variables|Default|SetOptionMenu _returnvalue))
  (UserInterface|Viewport|AddtoViewport _output_get 0)
  (Utilities|IsValid _refpause
    (:Is%20Valid
      (Variables|/Game/Widget/Menu/W_Pause.W_Pause_C|SetPause _refpause false))))

(event Custom|PauseMenuE
  (bind _optionmenu (Variables|Default|GetOptionMenu))
  (Viewport|RemoveAllWidgets)
  (bind _returnvalue (UserInterface|CreateWidget "/Game/Widget/Menu/W_Pause.W_Pause_C" self))
  (bind _output_get (Variables|Default|SetRefPause _returnvalue))
  (UserInterface|Viewport|AddtoViewport _output_get 0)
  (Utilities|IsValid _optionmenu
    (:Is%20Valid
      (Variables|/Game/Widget/Menu/W_Option.W_Option_C|SetOption? _optionmenu false))))

(event Custom|RemoveAllE
  (bind _refpause (Variables|Default|GetRefPause))
  (bind _optionmenu (Variables|Default|GetOptionMenu))
  (Viewport|RemoveAllWidgets)
  (Utilities|IsValid _refpause
    (:Is%20Valid
      (Widget|RemovefromParent _refpause))
    (:Is%20Not%20Valid
      _))
  (Utilities|IsValid _optionmenu
    (:Is%20Valid
      (Widget|RemovefromParent _optionmenu))))

(fn ConstructionScript)