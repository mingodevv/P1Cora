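; BP_MenuHero manages menu screens, switching between the main, collectible and option widgets.
; BeginPlay shows W_MainMenu, and three custom events handle moves from it to either submenu and back.
; Each switch checks the current widget reference, updates its state flag, removes all widgets, creates the target fresh, then clears the old reference.
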(event Custom|MainMenuE
  (Utilities|FlowControl|Sequence
    (:then_0
      (Utilities|IsValid (Variables|Default|GetCollectibleRef)
        (:Is%20Valid
          (Variables|/Game/Widget/Menu/W_Collectible.W_Collectible_C|SetCollect? (Variables|Default|GetCollectibleRef) false)
          (Viewport|RemoveAllWidgets)
          (bind _returnvalue (UserInterface|CreateWidget "/Game/Widget/Menu/W_MainMenu.W_MainMenu_C" (Game|GetPlayerController 0)))
          (bind _output_get (Variables|Default|SetMainMenuRef _returnvalue))
          (Variables|/Game/Widget/Menu/W_MainMenu.W_MainMenu_C|SetMenu _output_get true)
          (UserInterface|Viewport|AddtoViewport _output_get 0)
          (Variables|Default|SetCollectibleRef 0))))
    (:then_1
      (Utilities|IsValid (Variables|Default|GetOptionMenuRef)
        (:Is%20Valid
          (Variables|/Game/Widget/Menu/W_Option.W_Option_C|SetOption? (Variables|Default|GetOptionMenuRef) false)
          (Viewport|RemoveAllWidgets)
          (bind _returnvalue_2 (UserInterface|CreateWidget "/Game/Widget/Menu/W_MainMenu.W_MainMenu_C" (Game|GetPlayerController 0)))
          (bind _output_get_2 (Variables|Default|SetMainMenuRef _returnvalue_2))
          (Variables|/Game/Widget/Menu/W_MainMenu.W_MainMenu_C|SetMenu _output_get_2 true)
          (UserInterface|Viewport|AddtoViewport _output_get_2 0)
          (Variables|Default|SetOptionMenuRef 0))))))

(event Custom|OptionMenuE
  (Utilities|IsValid (Variables|Default|GetMainMenuRef)
    (:Is%20Valid
      (Variables|/Game/Widget/Menu/W_MainMenu.W_MainMenu_C|SetMenu (Variables|Default|GetMainMenuRef) false)
      (Viewport|RemoveAllWidgets)
      (bind _returnvalue (UserInterface|CreateWidget "/Game/Widget/Menu/W_Option.W_Option_C" (Game|GetPlayerController 0)))
      (bind _output_get (Variables|Default|SetOptionMenuRef _returnvalue))
      (Variables|/Game/Widget/Menu/W_Option.W_Option_C|SetOption? _output_get true)
      (UserInterface|Viewport|AddtoViewport _output_get 0)
      (Variables|Default|SetMainMenuRef 0))))

(event Custom|CollectibleMenuE
  (Utilities|IsValid (Variables|Default|GetMainMenuRef)
    (:Is%20Valid
      (Variables|/Game/Widget/Menu/W_MainMenu.W_MainMenu_C|SetMenu (Variables|Default|GetMainMenuRef) false)
      (Viewport|RemoveAllWidgets)
      (bind _returnvalue (UserInterface|CreateWidget "/Game/Widget/Menu/W_Collectible.W_Collectible_C" (Game|GetPlayerController 0)))
      (bind _output_get (Variables|Default|SetCollectibleRef _returnvalue))
      (UserInterface|Viewport|AddtoViewport _output_get 0)
      (Variables|Default|SetMainMenuRef 0))))

(event EventBeginPlay
  (bind _returnvalue (UserInterface|CreateWidget "/Game/Widget/Menu/W_MainMenu.W_MainMenu_C" (Game|GetPlayerController 0)))
  (bind _output_get (Variables|Default|SetMainMenuRef _returnvalue))
  (UserInterface|Viewport|AddtoViewport _output_get 0))

(fn ConstructionScript)