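; BP_GameMaster applies the player's saved music and effects volumes when play begins.
; BeginPlay checks the settings save slot and, if a save exists, loads it as BP_SaveSettings and copies its music and SFX values.
; AudioSetE then feeds those values into SCM_Audio as class overrides for SC_Music and SC_Effect and pushes the mix.
; Without a valid save, no audio changes are made.
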(event Custom|AudioSetE
  (Class|GameplayStatics|SetBaseSoundMix "/Game/Sound/SoundMix/SCM_Audio.SCM_Audio")
  (Audio|SetSoundMixClassOverride "/Game/Sound/SoundMix/SCM_Audio.SCM_Audio" "/Game/Sound/SoundClass/SC_Music.SC_Music" (Variables|Default|GetMusic%20Save) 1.0 1.0 true)
  (Audio|SetSoundMixClassOverride "/Game/Sound/SoundMix/SCM_Audio.SCM_Audio" "/Game/Sound/SoundClass/SC_Effect.SC_Effect" (Variables|Default|GetSFXsave) 1.0 1.0 true)
  (Audio|PushSoundMixModifier "/Game/Sound/SoundMix/SCM_Audio.SCM_Audio"))

(event EventBeginPlay
  (bind _returnvalue (SaveGame|DoesSaveGameExist (Variables|Base|GetSlot%20Name%20Setings)))
  (if _returnvalue
    (bind _returnvalue_2 (SaveGame|LoadGamefromSlot (Variables|Base|GetSlot%20Name%20Setings)))
    (bind _asbp_save_settings (Utilities|Casting|CastToBP_SaveSettings _returnvalue_2))
    (Variables|Default|SetMusic%20Save (Variables|/Game/Save/BP_SaveSettings.BP_SaveSettings_C|GetMusicSave _asbp_save_settings))
    (Variables|Default|SetSFXsave (Variables|/Game/Save/BP_SaveSettings.BP_SaveSettings_C|GetSFXsave _asbp_save_settings))
    (CallFunction|AudioSetE)))

(fn ConstructionScript)