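; BP_MovePoint is a monster-related Blueprint that holds a set of move points, apparently for monster movement.
; On BeginPlay it gathers eleven individual point variables into ArrayPoint in numbered order.
; It contains no movement or selection logic of its own, and its construction script is empty.
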(event EventBeginPlay
  (Variables|Default|SetArrayPoint (Utilities|Array|MakeArray (Variables|Default|GetPoint1) (Variables|Default|GetPoint2) (Variables|Default|GetPoint3) (Variables|Default|GetPoint4) (Variables|Default|GetPoint5) (Variables|Default|GetPoint6) (Variables|Default|GetPoint7) (Variables|Default|GetPoint8) (Variables|Default|GetPoint9) (Variables|Default|GetPoint10) (Variables|Default|GetPoint11))))

(fn ConstructionScript)