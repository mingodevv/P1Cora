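; BP_Monster is a patrolling monster that catches the hero and carries them back to the start point.
; MoveE loops delayed AI moves to random coordinates drawn from BP_MovePoint's point array.
; AI Perception triggers a chase of BP_Hero, or a move to any other stimulus location.
; On capture, View blocks new reactions while the input-disabled hero rides on PointPlayer to BP_StartPlayer, then is released as patrol resumes.
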(event OnTargetPerceptionUpdated(AIPerception)
  (params (Actor :type Actor%20Object%20Reference) (Stimulus :type AI%20Stimulus%20Structure))
  (bind _returnvalue (Math|Random|RandomIntegerinRange 0 10))
  (bind _movepoint (Variables|Default|GetMovePoint))
  (bind _startplayer (Variables|Default|GetStartPlayer))
  (bind _arraypoint (Variables|/Game/BP/Monster/BP_MovePoint.BP_MovePoint_C|GetArrayPoint _movepoint))
  (bind _pointstart (Variables|/Game/BP/Monster/BP_StartPlayer.BP_StartPlayer_C|GetPointStart _startplayer))
  (bind _returnvalue_2 (Transformation|GetWorldLocation _pointstart))
  (bind _output (Utilities|Array|Get(acopy) _arraypoint _returnvalue))
  (bind _returnvalue_3 (Transformation|GetWorldLocation _output))
  (bind (_x _y) (Math|Vector|BreakVector _returnvalue_3))
  (if (not (Variables|Default|GetView?))
    (bind _asbp_hero (Utilities|Casting|CastToBP_Hero Actor)
      (:then
        (AI|AIMoveTo self "0, 0, 0" _asbp_hero 1e+01 false
          (:OnSuccess
            (Default|StopAllInputE _asbp_hero)
            (Variables|Default|SetView? true)
            (Collision|SetActorEnableCollision _asbp_hero false)
            (Transformation|AttachComponentToComponent _asbp_hero (Variables|Default|GetPointPlayer) "None" "SnapToTarget" "SnapToTarget" "KeepWorld" true)
            (AI|AIMoveTo self (Math|Vector|MakeVector (.x _returnvalue_2) (.y _returnvalue_2) (.z (Transformation|GetActorLocation))) 0 5.0 false
              (:OnSuccess
                (Transformation|DetachFromActor _asbp_hero "KeepWorld" "KeepWorld" "KeepWorld")
                (Utilities|FlowControl|Sequence
                  (:then_0
                    (AI|AIMoveTo self (Math|Vector|MakeVector _x _y (.Z (Math|Vector|BreakVector (Transformation|GetActorLocation)))) 0 5.0 false
                      (:OnSuccess
                        (Variables|Default|SetView? false)
                        (CallFunction|MoveE))))
                  (:then_1
                    (Utilities|FlowControl|Delay 1.0)
                    (Default|EnableAllInputE _asbp_hero)
                    (Collision|SetActorEnableCollision _asbp_hero true))))))
          (:OnFail
            (CallFunction|MoveE))))
      (:CastFailed
        (AI|AIMoveTo self (.StimulusLocation (Utilities|Struct|BreakAIStimulus Stimulus)) 0 1e+01 false
          (:OnSuccess
            _)
          (:OnFail
            _))
        (CallFunction|MoveE)))))

(event Custom|MoveE
  (bind _returnvalue (Math|Random|RandomIntegerinRange 0 10))
  (bind _movepoint (Variables|Default|GetMovePoint))
  (bind _arraypoint (Variables|/Game/BP/Monster/BP_MovePoint.BP_MovePoint_C|GetArrayPoint _movepoint))
  (bind _output (Utilities|Array|Get(acopy) _arraypoint _returnvalue))
  (bind _returnvalue_2 (Transformation|GetWorldLocation _output))
  (bind (_x _y) (Math|Vector|BreakVector _returnvalue_2))
  (if (not (Variables|Default|GetView?))
    (Utilities|FlowControl|Delay 5.0)
    (AI|AIMoveTo self (Math|Vector|MakeVector _x _y (.Z (Math|Vector|BreakVector (Transformation|GetActorLocation)))) 0 1e+01 false
      (:OnSuccess
        (CallFunction|MoveE)))))

(event EventBeginPlay
  (bind _returnvalue (Actor|GetActorOfClass "/Game/BP/Monster/BP_MovePoint.BP_MovePoint_C"))
  (Variables|Default|SetMovePoint _returnvalue)
  (bind _returnvalue_2 (Actor|GetActorOfClass "/Game/BP/Monster/BP_StartPlayer.BP_StartPlayer_C"))
  (Variables|Default|SetStartPlayer _returnvalue_2)
  (Utilities|FlowControl|Delay 0.2)
  (CallFunction|MoveE))

(fn ConstructionScript)